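; BP_Potion is a collectible potion pickup that the first-person character gathers by overlapping its collision box.
; On overlap it increments the character's PotionsGet count and prints the new value to screen.
; When the count equals the character's PotionsMax the game pauses; otherwise the potion destroys itself and plays a 2D pickup sound.
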(event OnComponentBeginOverlap(Box_Collision)
  (params (OverlappedComponent :type Primitive%20Component%20Object%20Reference) (OtherActor :type Actor%20Object%20Reference) (OtherComp :type Primitive%20Component%20Object%20Reference) (OtherBodyIndex :type Integer) (bFromSweep :type Boolean) (SweepResult :type Hit%20Result%20Structure%20%28by%20ref%29))
  ;[0.15 0.15 0.15 0.5] add to potion count, play potion sound, potion disappears
  (bind _asbp_first_person_character (Utilities|Casting|CastToBP_FirstPersonCharacter OtherActor))
  (bind _result (Math|Integer|IncrementInt (Variables|/Game/FirstPerson/Blueprints/BP_FirstPersonCharacter.BP_FirstPersonCharacter_C|GetPotions_Get _asbp_first_person_character))
    (:%20%20
      (Development|PrintString (Utilities|String|ToString(Integer) _result))
      (if (== _result (Variables|/Game/FirstPerson/Blueprints/BP_FirstPersonCharacter.BP_FirstPersonCharacter_C|GetPotions_Max _asbp_first_person_character))
        (Game|SetGamePaused true)
        (else
          (Actor|DestroyActor)
          (Audio|PlaySound2D "/Game/SFX/Potion_SFX.Potion_SFX" 1.0 1.0 0.0 0 0))))))

(fn ConstructionScript)