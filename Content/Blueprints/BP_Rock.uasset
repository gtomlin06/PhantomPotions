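; BP_Rock is a boulder that the player can remove after collecting enough TNT.
; Overlapping its Box collision prints a one-time hint that the boulder is new and might be movable.
; Overlapping its StaticMesh casts to BP_FirstPersonCharacter, then destroys the rock if TNTGet equals TNTMax, or otherwise prints a hint about getting rid of it.
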(event OnComponentBeginOverlap(Box_Collision)
  (params (OverlappedComponent :type Primitive%20Component%20Object%20Reference) (OtherActor :type Actor%20Object%20Reference) (OtherComp :type Primitive%20Component%20Object%20Reference) (OtherBodyIndex :type Integer) (bFromSweep :type Boolean) (SweepResult :type Hit%20Result%20Structure%20%28by%20ref%29))
  ;[0.15 0.15 0.15 0.5] Rock hint 1x
  (Utilities|FlowControl|DoOnce false
    (:Completed
      (Development|PrintString "This boulder wasn't here before...I wonder if I could move it."))))

(event OnComponentBeginOverlap(StaticMesh)
  (params (OverlappedComponent :type Primitive%20Component%20Object%20Reference) (OtherActor :type Actor%20Object%20Reference) (OtherComp :type Primitive%20Component%20Object%20Reference) (OtherBodyIndex :type Integer) (bFromSweep :type Boolean) (SweepResult :type Hit%20Result%20Structure%20%28by%20ref%29))
  ;[0.15 0.15 0.15 0.5] destroy rock w/ tnt
  (bind _asbp_first_person_character (Utilities|Casting|CastToBP_FirstPersonCharacter OtherActor))
  (if (== (Variables|/Game/FirstPerson/Blueprints/BP_FirstPersonCharacter.BP_FirstPersonCharacter_C|GetTNT_Get _asbp_first_person_character) (Variables|/Game/FirstPerson/Blueprints/BP_FirstPersonCharacter.BP_FirstPersonCharacter_C|GetTNT_Max _asbp_first_person_character))
    (Actor|DestroyActor)
    (else
      (Development|PrintString "I wonder how I could get rid of it?"))))

(fn ConstructionScript)